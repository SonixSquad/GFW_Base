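; Gameplay ability that plays a directional hit reaction on an enemy.
; Once activated, it waits for the Enemy HitReact gameplay event and uses the instigator to cache hit direction vectors and resolve a direction name.
; It plays the hit react montage and jumps to the section matching that name, with optional debug prints.
; The graph never calls EndAbility.
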(event Ability|EventActivateAbility
  (bind _payload (Ability|Tasks|WaitGameplayEvent "(TagName=\"GFWTags.Events.Enemy.HitReact\")" 0)
    (:EventReceived
      (CallFunction|PrintDebugEventReceived _payload)
      (Class|GFWHitReact|CacheHitDirectionVectors (.Instigator (Utilities|Struct|BreakGameplayEventData _payload)))
      (Utilities|FlowControl|Sequence
        (:then_0
          ;[0.01338 0.02122 0.15 0.5] Cache HitDirection Name
          (Variables|Default|SetHitDirectionName (Class|GFWBlueprintLibrary|GetHitDirectionName (Class|GFWBlueprintLibrary|GetHitDirection (Variables|Default|GetAvatarForward) (Variables|Default|GetToInstigator))))
          ;[0.05478 0.02168 0.15 0.5] HitDirection Debug
          (Variables|Default|GetbDrawDebugs
            (:then
              (Development|PrintString (Utilities|String|ToString(Name) (Variables|Default|GetHitDirectionName))))
            (:else)))
        (:then_1
          (|PlayMontageandWaitProxy "None" (Variables|Default|GetHitReactMontage) 1.0 "None" true 1.0 0.0 false
            (:then
              (Ability|Animation|MontageJumptoSection (Variables|Default|GetHitDirectionName)))))))))

(event Ability|EventOnEndAbility
  (params (bWasCancelled :type Boolean)))

(fn PrintDebugEventReceived
  (params (GameplayEventData :type Gameplay%20Event%20Data%20Structure%20%28by%20ref%29))
  (Variables|Default|GetbDrawDebugs
    (:then
      (Development|PrintString (Utilities|String|Append "GA_GFW_HitReact Received From: " (Utilities|GetDisplayName (.Instigator (Utilities|Struct|BreakGameplayEventData GameplayEventData)))) true true "(R=1.000000,G=0.000000,B=0.041826,A=1.000000)" 0.5))
    (:else)))
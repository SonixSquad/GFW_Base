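; GA_GFW_Attack_Melee is an enemy melee attack gameplay ability for the Gameplay Ability System.
; On activation it plays a random montage from AttackMontages and ends when that montage completes, is interrupted or is cancelled.
; In parallel it waits once for a MeleeTraceHit event and draws a debug sphere at the impact point, applying no damage itself.
; Ending the ability sends an EndAttack event to the avatar actor.
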(event Ability|EventActivateAbility
  (Utilities|FlowControl|Sequence
    (:then_0
      (|PlayMontageandWaitProxy "None" (.OutItem (Utilities|Array|Random (Variables|Default|GetAttackMontages))) 1.0 "None" false 1.0 0.0 false
        (:OnCompleted
          _)
        (:OnInterrupted
          _)
        (:OnCancelled
          _))
      (Ability|EndAbility))
    (:then_1
      (bind _payload (Ability|Tasks|WaitGameplayEvent "(TagName=\"GFWTags.Events.Enemy.MeleeTraceHit\")" 0 true)
        (:EventReceived
          (Rendering|Debug|DrawDebugSphere (.impactpoint (Class|AbilitySystemBlueprintLibrary|EffectContextGetHitResult (.ContextHandle (Utilities|Struct|BreakGameplayEventData _payload)))) 3e+01 12 "(R=1.000000,G=1.000000,B=1.000000,A=1.000000)" 5.0))))))

(event Ability|EventOnEndAbility
  (params (bWasCancelled :type Boolean))
  (Ability|SendGameplayEventtoActor (Ability|GetAvatarActorfromActorInfo) "(TagName=\"GFWTags.Events.Enemy.EndAttack\")"))
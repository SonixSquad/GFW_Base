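; Gameplay Ability that drives enemy AI combat as a search, approach and attack loop.
; After a random per-enemy delay it finds the closest tagged actor, moves to it via the AI controller if it is alive, and searches again otherwise.
; It then rotates the enemy, waits out the rotation timeline and activates the attack ability by tag.
; An EndAttack gameplay event restarts the search.
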(event Custom|StartSearch
  (bind _returnvalue (Ability|GetAvatarActorfromActorInfo))
  (bind _bp_owning_enemy (Variables|Default|GetBP_Owning_Enemy))
  ;[0.15 0.15 0.15 0.5] Random Delay Between ATtacks
  (CallFunction|TargetSearchDebug false)
  (Variables|Default|GetBP_Owning_Enemy
    (:then
      (Ability|Tasks|WaitDelay (Math|Random|RandomFloatinRange (Variables|/Script/GAS_Base.GFW_EnemyCharacter|GetMinAttackDelay _bp_owning_enemy) (Variables|/Script/GAS_Base.GFW_EnemyCharacter|GetMaxAttackDelay _bp_owning_enemy))
        (:OnFinish
          (Utilities|FlowControl|Sequence
            (:then_0
              ;[0.15 0.15 0.15 0.5] Find closest Player Target
              (bind _returnvalue_2 (Class|GFWBlueprintLibrary|FindClosestActorwithTag _returnvalue (Transformation|GetActorLocation _returnvalue) (Variables|Default|GetTag)))
              (CallFunction|DebugTargetCharacter (.actor _returnvalue_2) false)
              (bind _asgfw_base_character (Utilities|Casting|CastToGFW_BaseCharacter (.actor _returnvalue_2)))
              (Variables|Default|SetTargetBaseCharacter _asgfw_base_character))
            (:then_1
              ;[0.15 0.15 0.15 0.5] Initiate Move to Target or Search again if Not Alive
              (Variables|Default|GetTargetBaseCharacter
                (:then
                  (Variables|/Script/GAS_Base.GFW_BaseCharacter|GetbAlive (Variables|Default|GetTargetBaseCharacter)
                    (:then
                      (CallFunction|MOvetoTargetandAttack))
                    (:else
                      (CallFunction|StartSearch))))
                (:else
                  (CallFunction|StartSearch))))))))
    (:else)))

(event Custom|MOveToTargetAndAttack
  ;[0.15 0.15 0.15 0.5] Move to Target
  (Variables|/Script/GAS_Base.GFW_BaseCharacter|GetbAlive (Variables|Default|GetBP_Owning_Enemy)
    (:then
      (bind _owning_ai_controller (Variables|Default|GetOwning_AI_Controller)
        (:then
          (AI|AIMoveTo _owning_ai_controller "0, 0, 0" (Variables|Default|GetTargetBaseCharacter) (Variables|/Script/GAS_Base.GFW_EnemyCharacter|GetAcceptanceRadius (Variables|Default|GetBP_Owning_Enemy)) "Default" "Default" true true
            (:OnMoveFinished
              (CallFunction|AttackTarget))))
        (:else)))
    (:else
      (CallFunction|StartSearch))))

(event Custom|AttackTarget
  ;[0.15 0.15 0.15 0.5] Rotate to Target and Wait till rotation is done
  (Default|RotatetoTarget (Variables|Default|GetBP_Owning_Enemy) (Variables|Default|GetTargetBaseCharacter))
  (Ability|Tasks|WaitDelay (Components|Timeline|GetTimelineLength (Variables|/Game/GAS_ToTW/Characters/Enemy/BP_GFW_EnemyBase.BP_GFW_EnemyBase_C|GetRotationTimeline (Variables|Default|GetBP_Owning_Enemy)))
    (:OnFinish
      ;[0.15 0.15 0.15 0.5] Actual Attack
      (Abilities|TryActivateAbilitiesbyTag (Ability|GetAbilitySystemComponentfromActorInfo) (GameplayTags|MakeGameplayTagContainerfromTag (GameplayTags|MakeLiteralGameplayTag "(TagName=\"GFWTags.GFWAbilities.Enemy.Attack\")")) true)
      (CallFunction|ShotTakenDebug true))))

(event Ability|EventActivateAbility
  (Utilities|FlowControl|Sequence
    (:then_0
      ;[0.15 0.15 0.15 0.5] Cache EnemyBAse and AI COntrollers
      (bind _asbp_gfw_enemy_base (Utilities|Casting|CastToBP_GFW_EnemyBase (Ability|GetAvatarActorfromActorInfo)))
      (bind _output_get (Variables|Default|SetBP_Owning_Enemy _asbp_gfw_enemy_base))
      (Variables|Default|SetOwning_AI_Controller (AI|GetAIController _output_get)))
    (:then_1
      ;[0.15 0.15 0.15 0.5] Search For Player Target
      (CallFunction|StartSearch))
    (:then_2
      ;[0.15 0.15 0.15 0.5] Wait for Gameplay Event [End Attack] before Starting new search
      (Ability|Tasks|WaitGameplayEvent "(TagName=\"GFWTags.Events.Enemy.EndAttack\")" 0
        (:EventReceived
          (CallFunction|StartSearch))))))

(fn DebugTargetCharacter
  (params (ClosestActor :type Actor%20Object%20Reference) (DEBUG? :type Boolean))
  (bind _returnvalue (Transformation|GetActorLocation ClosestActor))
  (bind _returnvalue_2 (+ _returnvalue "0.000000,0.000000,150.000000"))
  (Utilities|IsValid ClosestActor
    (:Is%20Valid
      (Variables|Default|SetbDrawDebugs DEBUG?)
      (Variables|Default|GetbDrawDebugs
        (:then
          (Rendering|Debug|DrawDebugSphere _returnvalue_2 5e+01 12 "(R=0.004959,G=1.000000,B=0.003036,A=1.000000)" 1e+01)
          (Development|PrintString (Utilities|String|ToString(Vector) _returnvalue_2) true true "(R=0.004959,G=1.000000,B=0.003036,A=1.000000)"))
        (:else
          _)))
    (:Is%20Not%20Valid
      (Development|PrintString "INVALID TARGET" true true "(R=0.578248,G=0.011027,B=1.000000,A=1.000000)")))
  (return))

(fn TargetSearchDebug
  (params (DEBUG%20? :type Boolean))
  (Variables|Default|SetbDrawDebugs DEBUG%20?)
  (Variables|Default|GetbDrawDebugs
    (:then
      (Development|PrintString "GA_GFW_SearchForTarget > Searching..."))
    (:else
      _))
  (return))

(fn ShotTakenDebug
  (params (DEBUG%20? :type Boolean))
  (Variables|Default|SetbDrawDebugs DEBUG%20?)
  (Variables|Default|GetbDrawDebugs
    (:then
      (Development|PrintString "SHOT TAKEN!" true true "(R=1.000000,G=0.000940,B=0.000045,A=1.000000)" 1.0))
    (:else
      _))
  (return))
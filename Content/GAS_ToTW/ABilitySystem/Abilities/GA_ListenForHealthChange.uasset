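; Gameplay ability that watches the avatar's health and triggers death when it runs out.
; On activation it starts an async attribute-change listener on the avatar's Ability System Component and keeps the task until the ability ends.
; Each change optionally prints the new value for debugging, and a value at or below zero activates abilities tagged as Death.
; The ability never ends itself, so it works as a persistent listener.
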(event Ability|EventActivateAbility
  (bind (_asynctaskproxy _attribute _newvalue) (|ListenforAttributeChange (Ability|GetAbilitySystemComponent (Ability|GetAvatarActorfromActorInfo)) "(AttributeName=\"Health\",Attribute=/Script/GAS_Base.GFW_AttributeSet:Health,AttributeOwner=\"/Script/CoreUObject.Class'/Script/GAS_Base.GFW_AttributeSet'\")")
    (:then
      (Variables|Default|SetAttributeChangeTask _asynctaskproxy))
    (:OnAttributeChanged
      (CallFunction|PrintHealthDebug _newvalue)
      (if (<= _newvalue 0.0)
        (Abilities|TryActivateAbilitiesbyTag (Ability|GetAbilitySystemComponentfromActorInfo) (GameplayTags|MakeGameplayTagContainerfromTag (GameplayTags|MakeLiteralGameplayTag "(TagName=\"GFWTags.GFWAbilities.Death\")")) true)))))

(event Ability|EventOnEndAbility
  (params (bWasCancelled :type Boolean))
  (bind _attributechangetask (Variables|Default|GetAttributeChangeTask)
    (:then
      (Class|GFWAttributeChangeTask|EndTask _attributechangetask))
    (:else)))

(fn PrintHealthDebug
  (params (InDouble :type Float%20%28double-precision%29))
  (Variables|Default|GetbDrawDebugs
    (:then
      (Development|PrintString (Utilities|String|Append "Health Now:" (Utilities|String|ToString(Float) InDouble)) true true "(R=1.000000,G=0.000940,B=0.000045,A=1.000000)"))
    (:else)))
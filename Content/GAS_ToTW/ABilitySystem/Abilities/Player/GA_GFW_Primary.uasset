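; Player primary attack gameplay ability that alternates between two attack montages through a FlipFlop and ends when the montage finishes or is interrupted.
; In parallel, it waits for the Primary gameplay event, then runs a hitbox overlap test and sends hit-react events to the actors found.
; Each hit actor receives GE_PlayerDamage at the ability's level.
; Helper functions handle debug printing and sphere drawing.
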(event Ability|EventActivateAbility
  (bind _returnvalue (Ability|GetAbilityLevel))
  (bind _returnvalue_2 (Ability|GetAbilitySystemComponentfromActorInfo))
  (bind _returnvalue_3 (Math|Conversions|ToFloat(Integer) _returnvalue))
  (Utilities|FlowControl|Sequence
    (:then_0
      ;[0.1454 0.15 0.02453 0.5] Ability goes here
      (Utilities|FlowControl|FlipFlop
        (:A
          ;;[0.02383 0.01243 0.15 0.5] Latent Task
          (|PlayMontageandWaitProxy "None" "/Game/GAS_ToTW/Characters/Anims/Primary/Player/AM_Primary_A1.AM_Primary_A1" 1.0 "None" true 1.0 0.0 false
            (:OnCompleted
              _)
            (:OnBlendOut
              _)
            (:OnInterrupted
              _)
            (:OnCancelled
              _)))
        (:B
          ;;[0.02383 0.01243 0.15 0.5] Latent Task
          (|PlayMontageandWaitProxy "None" "/Game/GAS_ToTW/Characters/Anims/Primary/Player/AM_Primary_B1.AM_Primary_B1" 1.0 "None" true 1.0 0.0 false
            (:OnCompleted
              _)
            (:OnBlendOut
              _)
            (:OnInterrupted
              _)
            (:OnCancelled
              _))))
      (Ability|EndAbility))
    (:then_1
      ;[0.2231 0.2292 0.05817 0.5] Respond to Gameplay Event Notify Tags - via Event Received
      (Ability|Tasks|WaitGameplayEvent "(TagName=\"GFWTags.Events.Player.Primary\")" 0
        (:EventReceived
          ;;[0.2231 0.2292 0.05817 0.5] Response Here
          (bind _returnvalue_4 (Class|GFWGAPrimary|HitBoxOverlapTest))
          (Class|GFWGAPrimary|SendHitReactEventtoActors _returnvalue_4)
          ;[0.004914 0 0.15 0.5] DEBUG
          (CallFunction|DebugHits false)
          ;[0.9699 1 0.1597 0.5] Apply GamePLayEffect - Damage
          (for _array_element _returnvalue_4
            (Variables|Default|GetbDrawDebugs
              (:then
                (Development|PrintString (Utilities|String|ToString(Float) _returnvalue_3) true true "(R=1.000000,G=0.000940,B=0.000045,A=1.000000)" 1e+01))
              (:else
                _))
            (GameplayEffects|ApplyGameplayEffectSpecToTarget _returnvalue_2 (GameplayEffects|MakeOutgoingSpec :self _returnvalue_2 :GameplayEffectClass "/Game/GAS_ToTW/ABilitySystem/GameplayEffects/Player/GE_PlayerDamage.GE_PlayerDamage_C" :Level _returnvalue_3) (Ability|GetAbilitySystemComponent _array_element))))))))

(event Ability|EventOnEndAbility
  (params (bWasCancelled :type Boolean)))

(fn EnableDebugs
  (params (DEBUG? :type Boolean))
  (bind _bdrawdebugs (Variables|Default|GetbDrawDebugs)
    (:then
      (Variables|Default|SetbDebugSphere _bdrawdebugs)
      (Variables|Default|GetbDebugAbilityStart
        (:then
          (Development|PrintString "GA_Primary_Activated" true true "(R=0.000000,G=1.000000,B=0.259747,A=1.000000)")
          (Variables|Default|SetbDebugAbilityStart false))
        (:else
          (Development|PrintString "GA_Primary_Ended" true true "(R=0.003639,G=0.036458,B=0.005480,A=1.000000)")
          (Variables|Default|SetbDebugAbilityStart true)
          (Variables|Default|SetbDebugSphere false))))
    (:else
      (return))))

(fn DebugHits
  (params (DEBUG%20? :type Boolean))
  (Variables|Default|SetbDrawDebugs DEBUG%20?)
  (Variables|Default|GetbDebugSphere
    (:then
      (Rendering|Debug|DrawDebugSphere (|DebugSphereCalc) (Variables|Default|GetRadius) 12 "(R=1.000000,G=1.000000,B=1.000000,A=1.000000)" 3.0))
    (:else
      (return))))
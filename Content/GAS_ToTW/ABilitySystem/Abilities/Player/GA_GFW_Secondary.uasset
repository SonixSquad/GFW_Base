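; GA_GFW_Secondary is a player Gameplay Ability for a secondary action, currently a placeholder with no gameplay effect.
; On activation it waits one second, then ends itself.
; Activation and end both call EnableDebugs, which, when DrawDebugs is on, prints an activated or ended message by flipping the DebugAbilityStart flag.
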(event Ability|EventActivateAbility
  ;[0.01079 0.01162 0.15 0.5] Enable Debug
  (CallFunction|EnableDebugs (Variables|Default|GetbDrawDebugs))
  (Utilities|FlowControl|Sequence
    (:then_0
      ;[0.1454 0.15 0.02453 0.5] Ability goes here
      (Utilities|FlowControl|Delay 1.0)
      (Ability|EndAbility))))

(event Ability|EventOnEndAbility
  (params (bWasCancelled :type Boolean))
  ;[0.01079 0.01162 0.15 0.5] Enable Debug
  (CallFunction|EnableDebugs (Variables|Default|GetbDrawDebugs)))

(fn EnableDebugs
  (params (DEBUG? :type Boolean))
  (Variables|Default|GetbDrawDebugs
    (:then
      (Variables|Default|GetbDebugAbilityStart
        (:then
          (Development|PrintString "GA_Secondary_Activated" true true "(R=0.050783,G=0.551754,B=1.000000,A=1.000000)")
          (Variables|Default|SetbDebugAbilityStart false))
        (:else
          (Development|PrintString "GA_Secondary_Ended" true true "(R=0.000000,G=0.005032,B=0.161458,A=1.000000)")
          (Variables|Default|SetbDebugAbilityStart true))))
    (:else
      (return))))
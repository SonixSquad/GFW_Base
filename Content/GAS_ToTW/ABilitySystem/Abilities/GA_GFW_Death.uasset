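; GA_GFW_Death is a Gameplay Ability that handles character death, playing DeathMontage while applying GE_Death.
; When the montage completes or aborts, RespawnCharacter picks melee or ranged enemy and spawn pad classes from identity tags and removes the Dead-tag effect.
; On authority it then ends the ability before destroying the ASC owner.
; Despite the name, nothing respawns: attribute reset, spawn-pad spawning and player-start teleport logic are all disconnected.
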(event Custom|RespawnCharacter
  (bind _returnvalue (Ability|GetAbilitySystemComponentfromActorInfo))
  (Utilities|FlowControl|Sequence
    (:then_0
      ;[0.05478 0.02168 0.15 0.5] Determine which enemy was killed and what to respawn
      (bind _returnvalue_2 (GameplayTags|HasMatchingGameplayTag(Message) _returnvalue "(TagName=\"GFWTags.Identity.Enemy.Melee\")"))
      (if _returnvalue_2
        (Variables|Default|SetEnemyType "/Game/GAS_ToTW/Characters/Enemy/BP_EnemyMelee.BP_EnemyMelee_C")
        (Variables|Default|SetSpawnPadType "/Game/GAS_ToTW/Actors/SpawnPads/BP_SpawnPad_Base_Enemy_Melee.BP_SpawnPad_Base_Enemy_Melee_C")
        (else
          (bind _returnvalue_3 (GameplayTags|HasMatchingGameplayTag(Message) _returnvalue "(TagName=\"GFWTags.Identity.Enemy.Ranged\")"))
          (if _returnvalue_3
            (Variables|Default|SetEnemyType "/Game/GAS_ToTW/Characters/Enemy/BP_EnemyRanged.BP_EnemyRanged_C")
            (Variables|Default|SetSpawnPadType "/Game/GAS_ToTW/Actors/SpawnPads/BP_SpawnPad_Base_Enemy_Ranged.BP_SpawnPad_Base_Enemy_Ranged_C")))))
    (:then_1
      ;[0.05478 0.02168 0.15 0.5] remove [DEAD] Gameplay Tags
      (Ability|RemoveGameplayEffectFromOwnerWithGrantedTags "(GameplayTags=((TagName=\"GFWTags.Status.Dead\")))" 1))
    (:then_2
      ;[0.3357 1 0] Cache BaseCharacter
      (bind _asgfw_base_character (Utilities|Casting|CastToGFW_BaseCharacter (Ability|GetAvatarActorfromActorInfo)))
      (Variables|Default|SetAs%20GFW%20Base%20Character _asgfw_base_character))
    (:then_5
      ;[0.3357 1 0] Destroy Actor, End ABility first to avoid crashes
      (Ability|HasAuthority
        (:True
          ;;[1 0 0.04183] Need to end the ability or the Attribute Reset does not work.
          (Ability|EndAbility)
          (Actor|DestroyActor (Components|GetOwner (Ability|GetAbilitySystemComponentfromActorInfo))))))))

(event Ability|EventActivateAbility
  (bind _returnvalue (Ability|GetAbilitySystemComponentfromActorInfo))
  ;[0.01338 0.02122 0.15 0.5] Play relevant Death Montage [specified in character BP] and respawn
  (|PlayMontageandWaitProxy "None" (Variables|Default|GetDeathMontage) 1.0 "Default" true 1.0 0.0 false
    (:then
      ;[0.05478 0.02168 0.15 0.5] Apply Gameplay Effect [Death]
      (GameplayEffects|ApplyGameplayEffectSpecToSelf _returnvalue (GameplayEffects|MakeOutgoingSpec :self _returnvalue :GameplayEffectClass "/Game/GAS_ToTW/ABilitySystem/GameplayEffects/GE_Death.GE_Death_C" :Level 1.0)))
    (:OnCompleted
      (CallFunction|RespawnCharacter :!label _label))
    (:OnInterrupted
      (goto _label))
    (:OnCancelled
      (goto _label))))
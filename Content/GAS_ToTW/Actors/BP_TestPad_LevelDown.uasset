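; Test pad actor that drops an overlapping actor's primary ability back to level 1.
; On box overlap it gets the actor's GFW_ASC and sets the level of GA_GFW_Primary directly, rather than decrementing it.
; For a BP_GFW_PlayerCharacter it also prints a level-down message and plays the level-up success montage on the character's mesh.
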(event OnComponentBeginOverlap(Box)
  (params (OverlappedComponent :type Primitive%20Component%20Object%20Reference) (OtherActor :type Actor%20Object%20Reference) (OtherComp :type Primitive%20Component%20Object%20Reference) (OtherBodyIndex :type Integer) (bFromSweep :type Boolean) (SweepResult :type Hit%20Result%20Structure%20%28by%20ref%29))
  (bind _asgfw_asc (Utilities|Casting|CastToGFW_ASC (Ability|GetAbilitySystemComponent OtherActor)))
  (Class|GFWASC|SetAbilityLevel _asgfw_asc "/Game/GAS_ToTW/ABilitySystem/Abilities/Player/GA_GFW_Primary.GA_GFW_Primary_C" 1)
  (bind _asbp_gfw_player_character (Utilities|Casting|CastToBP_GFW_PlayerCharacter OtherActor))
  (Development|PrintString "LEVELDOWN!" true true "(R=0.004959,G=1.000000,B=0.003036,A=1.000000)")
  (Animation|Montage|PlayMontage (Variables|/Script/Engine.Character|GetMesh _asbp_gfw_player_character) "/Game/GAS_ToTW/Characters/Anims/AM_LevelUpSuccess.AM_LevelUpSuccess"))

(event EventBeginPlay
  (|CallParentFunction) ; This node is disabled and will not be called.\nDrag off pins to build functionality.
)

(event Collision|EventActorBeginOverlap
  (params (OtherActor :type Actor%20Object%20Reference))
  (|CallParentFunction OtherActor) ; This node is disabled and will not be called.\nDrag off pins to build functionality.
)

(event EventTick
  (params (DeltaSeconds :type Float%20%28single-precision%29))
  (|CallParentFunction DeltaSeconds) ; This node is disabled and will not be called.\nDrag off pins to build functionality.
)

(fn ConstructionScript
  (|CallParentFunction))
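; Blueprint player character for a Gameplay Ability System project, adding debug hooks for testing enemies and ability levels.
; Keys 3 and 4 spawn ranged and melee enemies at the AISpawn component.
; The level-up test input casts the ability system component to GFW_ASC and sets the primary ability to a fixed level.
; Primary input is empty, with activation noted as implemented in C++; tag activation and level increment nodes remain disconnected.
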(event Input|EnhancedActionEvents|EnhancedInputActionIA_Primary
  (params (ActionValue :type Boolean) (ElapsedSeconds :type Float%20%28double-precision%29) (TriggeredSeconds :type Float%20%28double-precision%29) (InputAction :type Input%20Action%20Object%20Reference :default "/Game/GAS_ToTW/Input/Ability_Actions/IA_Primary.IA_Primary"))
  ;[0.0153 0.009564 0.15 0.5] BP Method to activate ability [already implemented in CPP]
  ;;[0.02614 0.01118 0.15 0.5] Connect to On Started
)

(event Input|EnhancedActionEvents|EnhancedInputActionIA_LevelUpTest
  (params (ActionValue :type Boolean) (ElapsedSeconds :type Float%20%28double-precision%29) (TriggeredSeconds :type Float%20%28double-precision%29) (InputAction :type Input%20Action%20Object%20Reference :default "/Game/GAS_ToTW/Input/Ability_Actions/IA_LevelUpTest.IA_LevelUpTest"))
  (:Started
    (bind _asgfw_asc (Utilities|Casting|CastToGFW_ASC (Ability|GetAbilitySystemComponent 0)))
    (Class|GFWASC|SetAbilityLevel _asgfw_asc "/Game/GAS_ToTW/ABilitySystem/Abilities/Player/GA_GFW_Primary.GA_GFW_Primary_C" 9)))

(event EventBeginPlay)

(event Collision|EventActorBeginOverlap
  (params (OtherActor :type Actor%20Object%20Reference)))

(event EventTick
  (params (DeltaSeconds :type Float%20%28single-precision%29)))

(event Input|KeyboardEvents|3
  (params (Key :type Key%20Structure :default "None"))
  (bind _ai_spawn (Variables|Default|GetAI_Spawn))
  (:Pressed
    (Game|SpawnActorfromClass "/Game/GAS_ToTW/Characters/Enemy/BP_EnemyRanged.BP_EnemyRanged_C" (Math|Transform|MakeTransform (Transformation|GetWorldLocation _ai_spawn) (Transformation|GetWorldRotation _ai_spawn) "1.000000,1.000000,1.000000") "AdjustIfPossibleButAlwaysSpawn" "MultiplyWithRoot" 0 0)))

(event Input|KeyboardEvents|4
  (params (Key :type Key%20Structure :default "None"))
  (bind _ai_spawn (Variables|Default|GetAI_Spawn))
  (:Pressed
    (Game|SpawnActorfromClass "/Game/GAS_ToTW/Characters/Enemy/BP_EnemyMelee.BP_EnemyMelee_C" (Math|Transform|MakeTransform (Transformation|GetWorldLocation _ai_spawn) (Transformation|GetWorldRotation _ai_spawn) "1.000000,1.000000,1.000000") "AdjustIfPossibleButAlwaysSpawn" "MultiplyWithRoot" 0 0)))

(fn ConstructionScript)
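; Heal pad Blueprint that adds the visual effects for a parent heal pad class; no healing logic lives here.
; SpawnHealEffects calls the parent, spawns the NS_HealFountain Niagara system at the HealEffectSpawn transform and stores it in HealFXRef.
; StopHealEffects deactivates that stored system without calling the parent.
; BeginPlay and construction only call the parent, while overlap and Tick are disabled.
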(event EventBeginPlay
  (|CallParentFunction))

(event Collision|EventActorBeginOverlap
  (params (OtherActor :type Actor%20Object%20Reference))
  (|CallParentFunction OtherActor) ; This node is disabled and will not be called.\nDrag off pins to build functionality.
)

(event EventTick
  (params (DeltaSeconds :type Float%20%28single-precision%29))
  (|CallParentFunction DeltaSeconds) ; This node is disabled and will not be called.\nDrag off pins to build functionality.
)

(event EventSpawnHealEffects
  (bind _healeffectspawn (Variables|Default|GetHealEffectSpawn))
  (|CallParentFunction)
  (bind _returnvalue (Niagara|SpawnSystematLocation "/Game/GAS_ToTW/FX/NS_HealFountain.NS_HealFountain" (Transformation|GetWorldLocation _healeffectspawn) (Transformation|GetWorldRotation _healeffectspawn)))
  (Variables|Default|SetHeal_FX_Ref _returnvalue))

(event EventStopHealEffects
  (Components|Activation|Deactivate (Variables|Default|GetHeal_FX_Ref)))

(fn ConstructionScript
  (|CallParentFunction))
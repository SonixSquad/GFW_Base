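; BP_Construct_GM spawns melee and ranged enemies at spawn pads on BeginPlay, with authority only.
; A RandomSpawn validity check selects between random-type spawning on SpawnPadType pads and type-specific spawning on melee and ranged pads.
; ChooseEnemyType picks melee or ranged for each random spawn.
; Each path spawns once per pad found, but at a randomly indexed pad from a hard-coded range, so locations can repeat.
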(event Custom|RandomSpawn
  (Networking|SwitchHasAuthority
    (:Authority
      (bind _spawnpadtype (Variables|Default|GetSpawnPadType)
        (:then
          ;[0.15 0.15 0.15 0.5] Random SPawn
          (bind _outactors (Actor|GetAllActorsOfClass _spawnpadtype))
          (for _array_element _outactors
            (bind _output_get (Variables|Default|SetEnemySpawnTransform (Transformation|GetActorTransform (Utilities|Array|Get(acopy) _outactors (Math|Random|RandomIntegerinRange 0 7)))))
            (CallFunction|ChooseEnemyType)
            (bind _enemytype (Variables|Default|GetEnemyType)
              (:then
                (Game|SpawnActorfromClass _enemytype _output_get "AdjustIfPossibleButAlwaysSpawn" "MultiplyWithRoot" 0 0))
              (:else
                (Development|PrintString "INVALID ENEMY TYPE" true true "(R=1.000000,G=0.000000,B=0.041826,A=1.000000)"))))
          (Development|PrintString "Spawns COmplete"))
        (:else)))))

(event Custom|SpawnSpecific
  (Networking|SwitchHasAuthority
    (:Authority
      (Utilities|FlowControl|Sequence
        (:then_0
          ;[0.15 0.15 0.15 0.5] Melee
          (bind _outactors (Actor|GetAllActorsOfClass "/Game/GAS_ToTW/Actors/SpawnPads/BP_SpawnPad_Base_Enemy_Melee.BP_SpawnPad_Base_Enemy_Melee_C"))
          (for _array_element _outactors
            (bind _output_get (Variables|Default|SetEnemySpawnTransform (Transformation|GetActorTransform (Utilities|Array|Get(acopy) _outactors (Math|Random|RandomIntegerinRange 0 7)))))
            (Game|SpawnActorfromClass "/Game/GAS_ToTW/Characters/Enemy/BP_EnemyMelee.BP_EnemyMelee_C" _output_get "AdjustIfPossibleButAlwaysSpawn" "MultiplyWithRoot" 0 0)))
        (:then_1
          ;[0.15 0.15 0.15 0.5] Ranged
          (bind _outactors_2 (Actor|GetAllActorsOfClass "/Game/GAS_ToTW/Actors/SpawnPads/BP_SpawnPad_Base_Enemy_Ranged.BP_SpawnPad_Base_Enemy_Ranged_C"))
          (for _array_element_2 _outactors_2
            (bind _output_get_2 (Variables|Default|SetEnemySpawnTransform (Transformation|GetActorTransform (Utilities|Array|Get(acopy) _outactors_2 (Math|Random|RandomIntegerinRange 0 7)))))
            (Game|SpawnActorfromClass "/Game/GAS_ToTW/Characters/Enemy/BP_EnemyRanged.BP_EnemyRanged_C" _output_get_2 "AdjustIfPossibleButAlwaysSpawn" "MultiplyWithRoot" 0 0)))))))

(event EventBeginPlay
  (Variables|Default|GetRandomSpawn?
    (:then
      (CallFunction|RandomSpawn))
    (:else
      (CallFunction|SpawnSpecific))))

(fn ConstructionScript)

(fn ChooseEnemyType
  (switch int (Math|Random|RandomIntegerinRange 1 2)
    (:1
      (Variables|Default|SetEnemyType "/Game/GAS_ToTW/Characters/Enemy/BP_EnemyMelee.BP_EnemyMelee_C"))
    (:2
      (Variables|Default|SetEnemyType "/Game/GAS_ToTW/Characters/Enemy/BP_EnemyRanged.BP_EnemyRanged_C"))))